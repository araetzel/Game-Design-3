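; BP_MovingWall is a puzzle gate wall that slides its door downward when OpenDoor is called.
; A timeline lerps the door's relative location and plays a world camera shake at the player controller's location on each update.
; Nodes for blending the camera to the wall and back are disconnected, so the NewViewTarget input goes unused.
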(event `OpenDoor`
  (params (NewViewTarget :type "Actor Object Reference"))
  (bind (_direction _newtrack_0) (`Timeline|Timeline`)
    (:`Update`
      (`SceneComponent.K2_SetRelativeLocation` (`self.Door`) (`KismetMathLibrary.VLerp` (0.0 0.0 0.0) (0.0 0.0 -400.0) _newtrack_0) false false)
      (`GameplayStatics.PlayWorldCameraShake` "/Game/Blueprints/PuzzleGate/CameraShake.CameraShake_C" (`self.K2_GetActorLocation` (`GameplayStatics.GetPlayerController` 0)) 0.0 2000.0))))

(fn `UserConstructionScript`)