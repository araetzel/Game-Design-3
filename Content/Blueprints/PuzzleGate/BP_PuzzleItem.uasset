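; BP_PuzzleItem is a pickup that counts toward the puzzle gate and can only be collected by the character whose PlayerControllerID is 0.
; On trigger overlap with that character, it calls CollectItem on the BP_PuzzleGate found by class lookup, plays a pickup sound and destroys itself.
; Any other BP_ThirdPersonCharacter gets a red on-screen warning instead.
; An unconnected copy of the collection logic remains in the graph.
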(event `self.Trigger.OnComponentBeginOverlap`
  (params (OverlappedComponent :type "PrimitiveComponent Object Reference") (OtherActor :type "Actor Object Reference") (OtherComp :type "PrimitiveComponent Object Reference") (OtherBodyIndex :type Integer) (bFromSweep :type Boolean) (SweepResult :type "HitResult Structure (by ref)"))
  (bind _asbp_third_person_character (cast `/Game/ThirdPerson/Blueprints/BP_ThirdPersonCharacter` OtherActor))
  (if (== (`/Game/ThirdPerson/Blueprints/BP_ThirdPersonCharacter.PlayerControllerID` _asbp_third_person_character) 0)
    (bind _returnvalue (`GameplayStatics.GetActorOfClass` "/Game/Blueprints/PuzzleGate/BP_PuzzleGate.BP_PuzzleGate_C"))
    (`/Game/Blueprints/PuzzleGate/BP_PuzzleGate.Collect Item` _returnvalue)
    (`GameplayStatics.PlaySound2D` "/Game/Audio/item-pick-up-38258.item-pick-up-38258" 1.0 1.0 0.0 null null)
    (`self.K2_DestroyActor`)
    (else
      (`KismetSystemLibrary.PrintString` "WARNING: You cannot pick up this type of item!" true true (struct :`R` 1.0 :`B` 0.045802 :`A` 1.0) 5.0))))

(fn `UserConstructionScript`)