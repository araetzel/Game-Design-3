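; BP_PuzzleGate is a door that opens once the player has collected the required number of items.
; CollectItem increments and prints the count, and OpenDoorCheck either fires OpenDoor once or prints a not-enough-items warning.
; A timeline swings the door's yaw open, adding a particle component every update and playing a sound once.
; The trigger overlap shows and hides an interact widget, created on BeginPlay, for the player character.
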(event `Open Door`
  (bind (_direction _doorrotation) (`Timeline|OpenDoor`)
    (:`Update`
      (`SceneComponent.K2_SetRelativeRotation` (`self.Door`) (`KismetMathLibrary.MakeRotator` 0.0 0.0 (`KismetMathLibrary.Lerp` 0.0 80.0 _doorrotation)) false false)
      (`AddComponent|NODE_AddParticleSystemComponent-0`)
      (`/Engine/EditorBlueprintResources/StandardMacros.DoOnce` false
        (:`Completed`
          (`GameplayStatics.PlaySound2D` "/Game/Audio/doorOpen_2.doorOpen_2" 1.0 1.0 0.0 null null))))))

(event `Collect Item`
  (`/Engine/EditorBlueprintResources/StandardMacros.IncrementInt` (`self.CurrentItemsCollected`)
    (:`  `
      (`KismetSystemLibrary.PrintString` (`KismetStringLibrary.Concat_StrStr` "You have collected " (`KismetStringLibrary.Conv_IntToString` (`self.CurrentItemsCollected`)) " items.") true true (struct :`G` 0.66 :`B` 1.0 :`A` 1.0) 5.0))))

(event `Open Door Check`
  (if (>= (`self.CurrentItemsCollected`) (`self.MaxItemsCollected`))
    (`/Engine/EditorBlueprintResources/StandardMacros.DoOnce` false
      (:`Completed`
        (`self.Open Door`)))
    (else
      (`KismetSystemLibrary.PrintString` "You need to collect all 5 items to open the door!" true true (struct :`R` 1.0 :`G` 0.007021 :`A` 1.0) 5.0))))

(event `self.Trigger.OnComponentBeginOverlap`
  (params (OverlappedComponent :type "PrimitiveComponent Object Reference") (OtherActor :type "Actor Object Reference") (OtherComp :type "PrimitiveComponent Object Reference") (OtherBodyIndex :type Integer) (bFromSweep :type Boolean) (SweepResult :type "HitResult Structure (by ref)"))
  (if (== OtherActor (`GameplayStatics.GetPlayerCharacter` 0))
    (`UserWidget.AddToPlayerScreen` (`self.InteractWidget`) 0)))

(event `self.Trigger.OnComponentEndOverlap`
  (params (OverlappedComponent :type "PrimitiveComponent Object Reference") (OtherActor :type "Actor Object Reference") (OtherComp :type "PrimitiveComponent Object Reference") (OtherBodyIndex :type Integer))
  (if (== (`GameplayStatics.GetPlayerCharacter` 0) OtherActor)
    (`Widget.RemoveFromParent` (`self.InteractWidget`))))

(event `self.ReceiveBeginPlay`
  (bind _returnvalue (`|CreateWidget` "/Game/Blueprints/PuzzleGate/W_Interact.W_Interact_C" (`GameplayStatics.GetPlayerControllerFromID` 0)))
  (set `self.InteractWidget` _returnvalue))

(fn `UserConstructionScript`)